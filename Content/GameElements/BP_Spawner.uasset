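; BP_Spawner is a building placement actor that spawns a BP_Building preview from a BuildingList row on BeginPlay.
; Each Tick moves the preview to the cursor trace hit and tints it red or green from the building's overlap event.
; ReleaseBuilding restores the saved material, calls StartConstruction and clears the reference, without itself checking for overlap.
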(event Custom|OnOverlapping
  (params (Overlapping :type Boolean))
  (Variables|Default|SetIsOverlaping Overlapping))

(event EventBeginPlay
  (bind _returnvalue (Game|SpawnActorfromClass "/Game/Buildings/BP_Building.BP_Building_C" (Math|Transform|MakeTransform "0, 0, 0" "0, 0, 0" "1.000000,1.000000,1.000000") "Undefined" "MultiplyWithRoot" 0 (Utilities|Struct|MakeDataTableRowHandle "/Game/Buildings/BuildingList.BuildingList" (Variables|Default|GetBuildingToSpawn)) 0))
  (bind _output_get (Variables|Default|SetPlacedBuilding _returnvalue))
  (EventDispatchers|BindEventtoOnOverlapping _output_get (delegate Custom|OnOverlapping))
  (Variables|Default|SetOriginalMaterial (Rendering|Material|GetMaterial (Variables|/Game/Buildings/BP_Building.BP_Building_C|GetBuildingMesh (Variables|Default|GetPlacedBuilding)) 0)))

(event EventTick
  (params (DeltaSeconds :type Float%20%28single-precision%29))
  (bind _my_player_controller (CallFunction|GetMyPlayerController))
  (bind _placedbuilding (Variables|Default|GetPlacedBuilding))
  (bind (_hitresult _returnvalue) (Game|Player|GetHitResultUnderCursorbyChannel _my_player_controller "TraceTypeQuery3" true))
  (bind _buildingmesh (Variables|/Game/Buildings/BP_Building.BP_Building_C|GetBuildingMesh _placedbuilding))
  (Variables|Default|GetPlacedBuilding
    (:then
      (if _returnvalue
        (Transformation|SetActorLocation (Variables|Default|GetPlacedBuilding) (.Location (Collision|BreakHitResult _hitresult)) false false)
        (if (Variables|Default|GetIsOverlaping)
          (Rendering|Material|SetMaterial _buildingmesh 0 "/Game/Buildings/Materials/RedBuilding.RedBuilding")
          (else
            (Rendering|Material|SetMaterial _buildingmesh 0 "/Game/Buildings/Materials/GreenBuilding.GreenBuilding")))))
    (:else)))

(fn ConstructionScript)

(fn ReleaseBuilding
  (Utilities|FlowControl|Sequence
    (:then_0
      (bind _placedbuilding (Variables|Default|GetPlacedBuilding)
        (:then
          (bind _originalmaterial (Variables|Default|GetOriginalMaterial)
            (:then
              (Rendering|Material|SetMaterial (Variables|/Game/Buildings/BP_Building.BP_Building_C|GetBuildingMesh _placedbuilding) 0 _originalmaterial))
            (:else)))
        (:else)))
    (:then_1
      (Default|StartConstruction (Variables|Default|GetPlacedBuilding))
      (Variables|Default|SetPlacedBuilding 0))))