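; BP_Building is a building actor that takes its mesh from a data table row in the construction script.
; Its BuildingBox overlaps broadcast OnOverlapping with true or false.
; StartConstruction plays a click, shows the Construction widget and starts a looping timer that advances progress, double-stepped for development.
; At full progress, FinishConstruction plays a tone, clears the timer and hides the widget.
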(event OnComponentBeginOverlap(BuildingBox)
  (params (OverlappedComponent :type Primitive%20Component%20Object%20Reference) (OtherActor :type Actor%20Object%20Reference) (OtherComp :type Primitive%20Component%20Object%20Reference) (OtherBodyIndex :type Integer) (bFromSweep :type Boolean) (SweepResult :type Hit%20Result%20Structure%20%28by%20ref%29))
  (Default|CallOnOverlapping true))

(event OnComponentEndOverlap(BuildingBox)
  (params (OverlappedComponent :type Primitive%20Component%20Object%20Reference) (OtherActor :type Actor%20Object%20Reference) (OtherComp :type Primitive%20Component%20Object%20Reference) (OtherBodyIndex :type Integer))
  (Default|CallOnOverlapping false))

(event EventBeginPlay)

(event Collision|EventActorBeginOverlap
  (params (OtherActor :type Actor%20Object%20Reference)))

(event EventTick
  (params (DeltaSeconds :type Float%20%28single-precision%29)))

(fn ConstructionScript
  (bind _buildingtype (Variables|Default|GetBuildingType))
  (bind (_datatable _rowname) (Utilities|Struct|BreakDataTableRowHandle _buildingtype))
  (bind _returnvalue (Utilities|GetDataTableRow _datatable _rowname)
    (:then
      (Components|StaticMesh|SetStaticMesh (Variables|Default|GetBuildingMesh) (.Mesh (Utilities|Struct|BreakSBuilding _returnvalue))))))

(fn StartConstruction
  (Audio|PlaySound2D "/Game/Interface_And_Item_Sounds/WAV/Click_06.Click_06" 1.0 1.0 0.0 0 0)
  (Development|SetHiddeninGame (Variables|Default|GetConstruction) false false)
  (Utilities|Time|SetTimerbyFunctionName 0 "UpdateConstructionProgress" 0.1 true))

(fn UpdateConstructionProgress
  (bind _result (Math|Integer|IncrementInt (Variables|Default|GetConstructionProgress))
    (:%20%20
      ;[0.15 0.15 0.15 0.5] faster for development
      (bind _result_2 (Math|Integer|IncrementInt _result)
        (:%20%20
          (Variables|Default|SetConstructionProgress _result_2)
          (bind _aswb_construction (Utilities|Casting|CastToWB_Construction (UserInterface|GetWidget (Variables|Default|GetConstruction))))
          (Default|UpdateProgress _aswb_construction (Variables|Default|GetConstructionProgress))
          (if (>= (Variables|Default|GetConstructionProgress) 100)
            (CallFunction|FinishConstruction)))))))

(fn FinishConstruction
  (Audio|PlaySound2D "/Engine/EngineSounds/1kSineTonePing.1kSineTonePing" 1.0 1.0 0.0 0 0)
  (Utilities|Time|ClearTimerbyFunctionName 0 "UpdateConstructionProgress")
  (Development|SetHiddeninGame (Variables|Default|GetConstruction) true false))